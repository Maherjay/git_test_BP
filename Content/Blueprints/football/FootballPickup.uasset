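; A grabbable physics football that BP_MotionController can pick up and release.
; Pickup turns off mesh physics simulation and attaches the root component to the given component, keeping its world transform.
; Drop restores simulation, detaches the actor, then sets a fixed angular velocity about Y and adds a small fixed linear velocity along Y.
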(event `/Game/VirtualRealityBP/Blueprints/PickupActorInterface.Pickup`
  (params (AttachTo :type "SceneComponent Object Reference"))
  (`PrimitiveComponent.SetSimulatePhysics` (`self.StaticMeshComponent`) false)
  (`SceneComponent.K2_AttachToComponent` (`self.K2_GetRootComponent`) AttachTo "None" "KeepWorld" "KeepWorld" "KeepWorld" false))

(event `/Game/VirtualRealityBP/Blueprints/PickupActorInterface.Drop`
  (bind _staticmeshcomponent (`self.StaticMeshComponent`))
  (`PrimitiveComponent.SetSimulatePhysics` (`self.StaticMeshComponent`) true)
  (`self.K2_DetachFromActor` "KeepWorld" "KeepWorld" "KeepWorld")
  (`PrimitiveComponent.SetPhysicsAngularVelocityInDegrees` _staticmeshcomponent (0.0 15.0 0.0) false "None")
  (`PrimitiveComponent.SetPhysicsLinearVelocity` _staticmeshcomponent (0.0 2.0 0.0) true "None"))

(fn `UserConstructionScript`)